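; Road generator actor that builds a spline road from data table coordinates in its construction script.
; Row names and the "z" and "y" columns become X, Y and Z points, scaled by 100, then added to the spline.
; A spline mesh is attached per segment, with shared mesh, roll, scale and optional collision.
; Arc tangent helper functions are defined but not called, and the event graph is inactive.
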(event EventBeginPlay)

(event Collision|EventActorBeginOverlap
  (params (OtherActor :type Actor%20Object%20Reference)))

(event EventTick
  (params (DeltaSeconds :type Float%20%28single-precision%29)))

(fn ConstructionScript
  (bind _spline (Variables|Default|GetSpline))
  (Utilities|FlowControl|Sequence
    (:then_0
      (|CollapseGraph_0))
    (:then_1
      (|addnodes))
    (:then_2
      (for _index (range 0 (- (Variables|Default|Getintsize) -2))
        (bind _returnvalue (AddComponent|AddSplineMeshComponent (Components|GetOwner (Variables|Default|GetSpline)) false))
        (bind _output_get (Variables|Default|SetLocal_currentSplineMesh _returnvalue))
        (Components|StaticMesh|SetStaticMesh _output_get (Variables|Default|GetLocal_trackElementMesh))
        (Transformation|AttachComponentToComponent _output_get _spline "None" "KeepRelative" "KeepRelative" "KeepRelative" true)
        (SplineMesh|SetStartandEnd _returnvalue (.Location (Spline|GetLocationandTangentatSplinePoint _spline _index "Local")) (.Tangent (Spline|GetLocationandTangentatSplinePoint _spline _index "Local")) (.Location (Spline|GetLocationandTangentatSplinePoint _spline (+ _index 1) "Local")) (.Tangent (Spline|GetLocationandTangentatSplinePoint _spline (+ _index 1) "Local")) true :!class /Script/Engine.SplineMeshComponent)
        (Class|SplineMeshComponent|SetStartRoll (Variables|Default|GetLocal_currentSplineMesh) (Variables|Default|GetLocal_startRoll) true)
        (Class|SplineMeshComponent|SetEndRoll (Variables|Default|GetLocal_currentSplineMesh) (Variables|Default|GetLocal_endRoll) true)
        (SplineMesh|SetStartScale (Variables|Default|GetLocal_currentSplineMesh) (Variables|Default|GetLocal_startScale) true :!class /Script/Engine.SplineMeshComponent)
        (SplineMesh|SetEndScale (Variables|Default|GetLocal_currentSplineMesh) (Variables|Default|GetLocal_endScale) true :!class /Script/Engine.SplineMeshComponent)
        (Collision|SetCollisionEnabled (Variables|Default|GetLocal_currentSplineMesh) (select (Variables|Default|Getcolisions) "QueryAndPhysics" "NoCollision"))))))

(fn Calculartangente
  (params (Raio :type Float%20%28single-precision%29) (Angulo :type Float%20%28single-precision%29))
  (return (Math|Vector|MakeVector (* Raio (Math|Trig|Cos(Degrees) Angulo)) (* (Math|Trig|Sin(Degrees) Angulo) Raio) 0.0)))

(fn Splinetangent
  (params (Raio :type Float%20%28single-precision%29) (StartAngle :type Float%20%28single-precision%29) (EndAngle :type Float%20%28single-precision%29))
  (bind _returnvalue (- EndAngle StartAngle))
  (bind _returnvalue_2 (+ _returnvalue 9e+01))
  (bind _returnvalue_3 (/ _returnvalue_2 1.552285))
  (bind _returnvalue_4 (* Raio _returnvalue_3))
  (bind _returnvalue_5 (Math|Conversions|ToVector(Float) _returnvalue_4))
  (bind _xz (CallFunction|Calculartangente Raio StartAngle))
  (bind _xz_2 (CallFunction|Calculartangente Raio EndAngle))
  (return _xz (* (Math|Vector|MakeVector (/ (.y (/ _xz Raio)) -1.0) (.x (/ _xz Raio)) 0.0) _returnvalue_5) _xz_2 (* (Math|Vector|MakeVector (/ (.y (/ _xz_2 Raio)) -1.0) (.x (/ _xz_2 Raio)) 0.0) _returnvalue_5)))