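; ConeSpline is a Blueprint that places copies of a preview mesh at regular spacing along a spline.
; Its construction script adds a scaled spline mesh component at each distance step and moves it to that world location, without setting spline deformation.
; A stored last index makes each pass start after the previously recorded final step.
; A separate function fills an array with the spaced locations but is not called here.
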(event EventBeginPlay)

(fn ConstructionScript
  (CallFunction|CreateMeshsesAlongSpline))

(fn CreateSplineLocationArray
  (Utilities|Array|Clear (Variables|Default|Getlocat))
  (for _index (range 0 (.ReturnValue (Math|Float|Division(WholeandRemainder) (Spline|GetSplineLength (Variables|Default|GetSpline)) (Variables|Default|GetSpacing))))
    (Utilities|Array|Add (Variables|Default|Getlocat) (Spline|GetLocationatDistanceAlongSpline (Variables|Default|GetSpline) (* _index (Variables|Default|GetSpacing)) "World"))))

(fn CreateMeshsesAlongSpline
  (bind _spline (Variables|Default|GetSpline))
  (bind _spacing (Variables|Default|GetSpacing))
  (bind _returnvalue (Spline|GetSplineLength _spline))
  (bind _returnvalue_2 (Math|Float|Division(WholeandRemainder) _returnvalue _spacing))
  (Variables|Default|SetLastBeforeInd _returnvalue_2)
  (for _index (range (stale _output_get) _returnvalue_2)
    (bind _returnvalue_3 (AddComponent|AddSplineMeshComponent false (Math|Transform|MakeTransform (Spline|GetLocationatDistanceAlongSpline (Variables|Default|GetSpline) (* _index (Variables|Default|GetSpacing)) "World") "0, 0, 0" "0.300000,0.300000,1.250000")))
    (Components|StaticMesh|SetStaticMesh _returnvalue_3 "/Game/Geometry/Meshes/CubePreview.CubePreview")
    (Transformation|SetWorldLocation _returnvalue_3 (Spline|GetLocationatDistanceAlongSpline (Variables|Default|GetSpline) (* _index (Variables|Default|GetSpacing)) "World") false false)
    (LocalVariables|SetLastLocation (Spline|GetLocationatDistanceAlongSpline (Variables|Default|GetSpline) (* _index (Variables|Default|GetSpacing)) "World")))
  (bind _output_get (Variables|Default|SetLastInd (+ _returnvalue_2 1))))