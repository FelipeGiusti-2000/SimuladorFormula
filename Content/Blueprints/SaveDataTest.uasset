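; Test actor that saves and restores the placed Cone actors through a MySaveGame slot.
; SaveConeData writes every Cone's actor reference and transform into parallel arrays in a new save object, then prints success or failure.
; LoadConeData loops over the saved references only for indices, spawning a fresh Cone at each stored transform without removing existing ones.
; Neither event is called within this Blueprint.
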(event Custom|SaveConeData
  ;[0.4434 0.9181 1] Save/Load
  ;;[1 1 1] save game
  (bind _returnvalue (SaveGame|CreateSaveGameObject "/Game/Blueprints/MySaveGame.MySaveGame_C"))
  (bind _output_get (Variables|Default|SetSaveGameSubClass _returnvalue))
  (bind _asmy_save_game (Utilities|Casting|CastToMySaveGame _output_get))
  (bind _outactors (Actor|GetAllActorsOfClass "/Game/Blueprints/Cone.Cone_C"))
  (for _array_element _outactors
    (Utilities|FlowControl|Sequence
      (:then_0
        (Utilities|Array|Add (Variables|/Game/Blueprints/MySaveGame.MySaveGame_C|GetconeClassArraySave _asmy_save_game) _array_element))
      (:then_1
        (Utilities|Array|Add (Variables|/Game/Blueprints/MySaveGame.MySaveGame_C|GetconeTransformArray _asmy_save_game) (Transformation|GetActorTransform _array_element)))))
  (bind _returnvalue_2 (SaveGame|SaveGametoSlot (Variables|Default|GetSaveGameSubClass) (Variables|Default|GetSaveGameString)))
  (if _returnvalue_2
    (Development|PrintString "Save Complete")
    (else
      (Development|PrintString "Save Failed" true true "(R=1.000000,G=0.082348,B=0.154047,A=1.000000)"))))

(event Custom|LoadConeData
  ;[0.4434 0.9181 1] Save/Load
  ;;[1 1 1] load game
  (bind _returnvalue (SaveGame|DoesSaveGameExist (Variables|Default|GetSaveGameString)))
  (if _returnvalue
    (bind _returnvalue_2 (SaveGame|LoadGamefromSlot (Variables|Default|GetSaveGameString)))
    (bind _output_get (Variables|Default|SetSaveGameSubClass _returnvalue_2))
    (bind _asmy_save_game (Utilities|Casting|CastToMySaveGame _output_get))
    (for (_ _array_index) (Variables|/Game/Blueprints/MySaveGame.MySaveGame_C|GetconeClassArraySave _asmy_save_game)
      (Game|SpawnActorfromClass "/Game/Blueprints/Cone.Cone_C" (Utilities|Array|Get(acopy) (Variables|/Game/Blueprints/MySaveGame.MySaveGame_C|GetconeTransformArray _asmy_save_game) _array_index) "Undefined" 0 0))
    (else
      (Development|PrintString "Save does not exist"))))

(event EventBeginPlay)

(event Collision|EventActorBeginOverlap
  (params (OtherActor :type Actor%20Object%20Reference)))

(event EventTick
  (params (DeltaSeconds :type Float%20%28single-precision%29)))

(fn ConstructionScript)