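; Track generator Blueprint that builds a road along a spline in its construction script, optionally looping back to the first point.
; It resizes a per-point road data array to match the spline point count, filling new entries from defaults.
; Each segment becomes a spline mesh, interpolating bank, width and thickness between neighboring points, with switchable collision.
; An optional debug pass labels each point with its index as 3D text.
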(fn ConstructionScript
  (Utilities|FlowControl|Sequence
    (:then_0
      (|Storenumberofsplinepoints))
    (:then_1
      (|BuildRoadDataarray))
    (:then_2
      (|constructionloop))
    (:then_3
      (if (Variables|Default|GetdrawTrackPointNumbers)
        (for _index (range 0 (- (Variables|Default|GetnumberOfSplinePoints) 1))
          (Variables|Default|SetcurrentTrackPoint (Utilities|String|ToString(Integer) _index))
          (bind _returnvalue (AddComponent|AddTextRenderComponent false (Math|Transform|MakeTransform (Math|Vector|MakeVector (.X (Math|Vector|BreakVector (.Location (Spline|GetLocationandTangentatSplinePoint (Variables|Default|GetSpline) _index "Local")))) (.Y (Math|Vector|BreakVector (.Location (Spline|GetLocationandTangentatSplinePoint (Variables|Default|GetSpline) _index "Local")))) (+ (.Z (Math|Vector|BreakVector (.Location (Spline|GetLocationandTangentatSplinePoint (Variables|Default|GetSpline) _index "Local")))) 5e+01)) (Math|Conversions|RotationFromXVector (* (.Tangent (Spline|GetLocationandTangentatSplinePoint (Variables|Default|GetSpline) _index "Local")) -1)))))
          (Rendering|Components|TextRender|SetText _returnvalue (Utilities|Text|ToText(String) (Variables|Default|GetcurrentTrackPoint))))))))

(fn BuildTrackElement
  (params (loopIndex :type Integer) (trackElementMesh :type Static%20Mesh%20Object%20Reference))
  (LocalVariables|SetLocal_currentLoopIndex loopIndex)
  (LocalVariables|SetLocal_nextLoopIndex (Math|Integer|%(Integer) (+ loopIndex 1) (Variables|Default|GetnumberOfSplinePoints)))
  (LocalVariables|SetLocal_trackElementMesh trackElementMesh)
  (Utilities|FlowControl|Sequence
    (:then_0
      (LocalVariables|SetLocal_startLocation (.Location (Spline|GetLocationandTangentatSplinePoint (Variables|Default|GetSpline) (LocalVariables|GetLocal_currentLoopIndex) "Local")))
      (LocalVariables|SetLocal_startTangent (.Tangent (Spline|GetLocationandTangentatSplinePoint (Variables|Default|GetSpline) (LocalVariables|GetLocal_currentLoopIndex) "Local")))
      (LocalVariables|SetLocal_endLocation (.Location (Spline|GetLocationandTangentatSplinePoint (Variables|Default|GetSpline) (LocalVariables|GetLocal_nextLoopIndex) "Local")))
      (LocalVariables|SetLocal_endTangent (.Tangent (Spline|GetLocationandTangentatSplinePoint (Variables|Default|GetSpline) (LocalVariables|GetLocal_nextLoopIndex) "Local")))
      (LocalVariables|SetLocal_startRoll (.trackbank (Utilities|Array|Get(acopy) (Variables|Default|GetroadDataArray) (LocalVariables|GetLocal_currentLoopIndex))))
      (LocalVariables|SetLocal_startScale (Math|Vector2D|MakeVector2D (.trackwidth (Utilities|Array|Get(acopy) (Variables|Default|GetroadDataArray) (LocalVariables|GetLocal_currentLoopIndex))) (.trackthicness (Utilities|Array|Get(acopy) (Variables|Default|GetroadDataArray) (LocalVariables|GetLocal_currentLoopIndex)))))
      (LocalVariables|SetLocal_endRoll (.trackbank (Utilities|Array|Get(acopy) (Variables|Default|GetroadDataArray) (LocalVariables|GetLocal_nextLoopIndex))))
      (LocalVariables|SetLocal_endScale (Math|Vector2D|MakeVector2D (.trackwidth (Utilities|Array|Get(acopy) (Variables|Default|GetroadDataArray) (LocalVariables|GetLocal_nextLoopIndex))) (.trackthicness (Utilities|Array|Get(acopy) (Variables|Default|GetroadDataArray) (LocalVariables|GetLocal_nextLoopIndex))))))
    (:then_1
      (bind _returnvalue (AddComponent|AddSplineMeshComponent false))
      (LocalVariables|SetLocal_currentSplineMesh _returnvalue)
      (Components|StaticMesh|SetStaticMesh (LocalVariables|GetLocal_currentSplineMesh) (LocalVariables|GetLocal_trackElementMesh))
      (SplineMesh|SetStartandEnd (LocalVariables|GetLocal_currentSplineMesh) (LocalVariables|GetLocal_startLocation) (LocalVariables|GetLocal_startTangent) (LocalVariables|GetLocal_endLocation) (LocalVariables|GetLocal_endTangent) true :!class /Script/Engine.SplineMeshComponent)
      (Class|SplineMeshComponent|SetStartRoll (LocalVariables|GetLocal_currentSplineMesh) (LocalVariables|GetLocal_startRoll) true)
      (Class|SplineMeshComponent|SetEndRoll (LocalVariables|GetLocal_currentSplineMesh) (LocalVariables|GetLocal_endRoll) true)
      (SplineMesh|SetStartScale (LocalVariables|GetLocal_currentSplineMesh) (LocalVariables|GetLocal_startScale) true :!class /Script/Engine.SplineMeshComponent)
      (SplineMesh|SetEndScale (LocalVariables|GetLocal_currentSplineMesh) (LocalVariables|GetLocal_endScale) true :!class /Script/Engine.SplineMeshComponent)
      (Collision|SetCollisionEnabled (LocalVariables|GetLocal_currentSplineMesh) (select (Variables|Default|Getcolisions) "QueryAndPhysics" "NoCollision")))))